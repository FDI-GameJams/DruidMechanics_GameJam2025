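; BP_AffectableArea is a trigger volume that changes its space layout when the player performs their special ability inside it.
; On BeginPlay it registers each BP_AffectableObject already overlapping its box via AddAffectableObject, printing names for debugging.
; It binds to the player's ability-performed delegate on begin overlap and unbinds on end overlap.
; That delegate calls ChangeSpaceLayout, which, like AddAffectableObject, is defined outside this graph.
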(event `self.ReceiveBeginPlay`
  (for _array_element (`PrimitiveComponent.GetOverlappingActors` (`self.BoxCollisionComponent`) "/Game/GameJam/Blueprints/Affectables/BP_AffectableObject.BP_AffectableObject_C")
    (bind _asbp_affectable_object (cast `/Game/GameJam/Blueprints/Affectables/BP_AffectableObject` _array_element))
    (`self.AddAffectableObject` _asbp_affectable_object)
    (`KismetSystemLibrary.PrintString` (`KismetSystemLibrary.GetDisplayName` _array_element))))

(event `self.BoxCollisionComponent.OnComponentBeginOverlap`
  (params (OverlappedComponent :type "PrimitiveComponent Object Reference") (OtherActor :type "Actor Object Reference") (OtherComp :type "PrimitiveComponent Object Reference") (OtherBodyIndex :type Integer) (bFromSweep :type Boolean) (SweepResult :type "HitResult Structure (by ref)"))
  ; Listen to Ability Performed Event broadcasted from player when overlapping, unbind from it when not overlapping
  (if (== (`GameplayStatics.GetObjectClass` OtherActor) "/Game/GameJam/Blueprints/Player/BP_Player.BP_Player_C")
    (bind _asbp_player (cast `/Game/GameJam/Blueprints/Player/BP_Player` OtherActor))
    (add `SpecialAbilityComponent.OnAbilityPerformedDelegate` (`/Game/GameJam/Blueprints/Player/BP_Player.Special Ability` _asbp_player) (delegate `CustomEvent`))))

(event `CustomEvent`
  ; Listen to Ability Performed Event broadcasted from player when overlapping, unbind from it when not overlapping
  (`self.ChangeSpaceLayout`))

(event `self.BoxCollisionComponent.OnComponentEndOverlap`
  (params (OverlappedComponent :type "PrimitiveComponent Object Reference") (OtherActor :type "Actor Object Reference") (OtherComp :type "PrimitiveComponent Object Reference") (OtherBodyIndex :type Integer))
  ; Listen to Ability Performed Event broadcasted from player when overlapping, unbind from it when not overlapping
  (if (== (`GameplayStatics.GetObjectClass` OtherActor) "/Game/GameJam/Blueprints/Player/BP_Player.BP_Player_C")
    (remove `SpecialAbilityComponent.OnAbilityPerformedDelegate` (`/Game/GameJam/Blueprints/Player/BP_Player.Special Ability` (stale `self.BoxCollisionComponent.OnComponentBeginOverlap` _asbp_player)) (delegate `CustomEvent`))))

(fn `UserConstructionScript`)